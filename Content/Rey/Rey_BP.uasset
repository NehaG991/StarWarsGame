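; Rey character Blueprint that handles toggling a lightsaber and a basic two-hit melee combo.
; The G key flips Ignited, playing the matching ignite or deactivate animation and attached sound on the Saber.
; Left mouse alternates two attack montages through ComboCount, which a retriggerable delay resets after a pause.
; An Attacking flag gates new attacks, though this graph never clears it and attacks ignore the Ignited state.
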(event `Key|G`
  (params (Key :type "Key Structure"))
  ;[1 1 1] Ignite/Deactive Saber Code
  (:`Pressed`
    (if (`self.Ignited`)
      (`SkeletalMeshComponent.PlayAnimation` (`self.Saber`) "/Game/Rey/Saber/DeactivateSaber.DeactivateSaber" false)
      (`GameplayStatics.SpawnSoundAttached` "/Game/Rey/Sounds/Lightsaber_Powering_Down_Sound_Effect.Lightsaber_Powering_Down_Sound_Effect" (`self.Saber`) "None" (0.0 0.0 0.0) (struct) "KeepRelativeOffset" false 1.0 1.0 0.0 null null)
      (set `self.Ignited` false)
      (else
        (`SkeletalMeshComponent.PlayAnimation` (`self.Saber`) "/Game/Rey/Saber/IgniteSaber.IgniteSaber" false)
        (`GameplayStatics.SpawnSoundAttached` "/Game/Rey/Sounds/Lightsaber_Igniting_Sound_Effect.Lightsaber_Igniting_Sound_Effect" (`self.Saber`) "None" (0.0 0.0 0.0) (struct) "KeepRelativeOffset" false 1.0 1.0 0.0 null null)
        (set `self.Ignited` true)))))

(event `self.ReceiveBeginPlay`)

(event `InputAction|LMBDown`
  (params (Key :type "Key Structure"))
  ;[1 1 1] Basic Combo System
  (:`Pressed`
    (if (not (`self.bAttacking`))
      (set `self.bAttacking` true)
      (switch `int` (`self.ComboCount`)
        (:`0`
          (`self.PlayAnimMontage` "/Game/Rey/Animations/Attack1Montage.Attack1Montage" 2.0)
          (set `self.ComboCount` 1))
        (:`1`
          (`self.PlayAnimMontage` "/Game/Rey/Animations/Attack2Montage.Attack2Montage")
          (set `self.ComboCount` 0)))
      (`KismetSystemLibrary.RetriggerableDelay` 1.5)
      (set `self.ComboCount` 0))))

(fn `UserConstructionScript`)